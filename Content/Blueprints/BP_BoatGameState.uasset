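; Game state for the powerboat game that sets up the HUD and opens the completion and pause screens.
; On BeginPlay it finds the docking area, sets game-only input, adds the HUD and binds to the docking area's PlayerDocked and the player powerboat's PauseGame events.
; Completion and pause each add their widget and switch to UI-only input with a visible cursor; pausing also pauses the game.
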(event Custom|Open%20End%20Screen
  (bind _returnvalue (Game|GetPlayerController 0))
  (EventDispatchers|UnbindEventfromPlayerDocked (Variables|Default|GetDockingArea) (delegate Custom|Open%20End%20Screen))
  (Development|PrintString "Completed and Docked")
  (bind _returnvalue_2 (UserInterface|CreateWidget "/Game/UI/W_CompletionScreen.W_CompletionScreen_C"))
  (UserInterface|Viewport|AddtoViewport _returnvalue_2 1)
  (Variables|/Script/Engine.PlayerController|SetbShowMouseCursor _returnvalue true)
  (Input|SetInputModeUIOnly _returnvalue _returnvalue_2 "DoNotLock" false))

(event Custom|Pause%20Game
  (bind _returnvalue (Game|GetPlayerController 0))
  (bind _returnvalue_2 (UserInterface|CreateWidget "/Game/UI/W_PauseScreen.W_PauseScreen_C"))
  (UserInterface|Viewport|AddtoViewport _returnvalue_2 1)
  (Game|SetGamePaused true)
  (Variables|/Script/Engine.PlayerController|SetbShowMouseCursor _returnvalue true)
  (Input|SetInputModeUIOnly _returnvalue _returnvalue_2 "DoNotLock" false))

(event EventBeginPlay
  (bind _returnvalue (Game|GetPlayerController 0))
  (bind _returnvalue_2 (Actor|GetActorOfClass "/Game/Gameplay/DockingArea/BP_DockingArea.BP_DockingArea_C"))
  (bind _output_get (Variables|Default|SetDockingArea _returnvalue_2))
  (EventDispatchers|BindEventtoPlayerDocked _output_get (EventDispatchers|CreateEvent :!event Custom|Open%20End%20Screen))
  (Input|SetInputModeGameOnly _returnvalue true)
  (Variables|/Script/Engine.PlayerController|SetbShowMouseCursor _returnvalue false)
  (bind _returnvalue_3 (UserInterface|CreateWidget "/Game/UI/W_HUD.W_HUD_C"))
  (UserInterface|Viewport|AddtoViewport _returnvalue_3 0)
  (bind _asbp_powerboat (Utilities|Casting|CastToBP_Powerboat (Game|Player|GetPlayerPawn 0)))
  (EventDispatchers|BindEventtoPauseGame _asbp_powerboat (EventDispatchers|CreateEvent :!event Custom|Pause%20Game)))

(fn ConstructionScript)