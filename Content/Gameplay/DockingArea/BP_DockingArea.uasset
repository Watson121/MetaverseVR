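; Docking zone actor that detects when a BP_Powerboat stops inside it and signals that the player has docked.
; Mesh overlap recolours the highlighter green or red through a dynamic material instance and shows or hides the docking widget.
; While occupied, Tick queries the player pawn's movement, counting down when stationary and calling PlayerDocked at zero.
; Movement resets the timer and shows the widget's stop box.
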(event OnComponentBeginOverlap(DockingAreaMesh)
  (params (OverlappedComponent :type Primitive%20Component%20Object%20Reference) (OtherActor :type Actor%20Object%20Reference) (OtherComp :type Primitive%20Component%20Object%20Reference) (OtherBodyIndex :type Integer) (bFromSweep :type Boolean) (SweepResult :type Hit%20Result%20Structure%20%28by%20ref%29))
  ;[0 0 0] Checking if Powerboat is in range
  (Utilities|Casting|CastToBP_Powerboat OtherActor)
  (CallFunction|UpdateHighlighterMaterial "(R=0.045569,G=1.000000,B=0.000000,A=1.000000)")
  (Development|SetHiddeninGame (Variables|Default|GetDockingAreaWidget) false false)
  (Variables|Default|SetPowerboatInArea true))

(event OnComponentEndOverlap(DockingAreaMesh)
  (params (OverlappedComponent :type Primitive%20Component%20Object%20Reference) (OtherActor :type Actor%20Object%20Reference) (OtherComp :type Primitive%20Component%20Object%20Reference) (OtherBodyIndex :type Integer))
  ;[0 0 0] Checking if Powerboat is in range
  (Utilities|Casting|CastToBP_Powerboat OtherActor)
  (CallFunction|UpdateHighlighterMaterial "(R=1.000000,G=0.007519,B=0.000000,A=1.000000)")
  (Development|SetHiddeninGame (Variables|Default|GetDockingAreaWidget) true false)
  (Variables|Default|SetPowerboatInArea false))

(event EventBeginPlay
  (Development|SetHiddeninGame (Variables|Default|GetDockingAreaWidget) true false)
  (Variables|Default|SetMAX_COUNTDOWN_TIMER (Variables|Default|GetCountdownTimer)))

(event EventTick
  (params (DeltaSeconds :type Float%20%28single-precision%29))
  ;[0 0 0] Countdown Timer
  (if (Variables|Default|GetPowerboatInArea)
    (bind _ismoving (Class|BPIPowerboat|IsMoving(Message) (Game|Player|GetPlayerPawn 0)))
    (if (not _ismoving)
      (bind _output_get (Variables|Default|SetCountdownTimer (Math|Interpolation|FInterptoConstant (Variables|Default|GetCountdownTimer) 0.0 DeltaSeconds 1.0)))
      (bind _asw_docking_area (Utilities|Casting|CastToW_DockingArea (UserInterface|GetWidget (Variables|Default|GetDockingAreaWidget))))
      (Default|ShowCountdownTimer _asw_docking_area _output_get)
      (if (== _output_get 0.0)
        (Default|CallPlayerDocked))
      (else
        (Variables|Default|SetCountdownTimer (Variables|Default|GetMAX_COUNTDOWN_TIMER))
        (bind _asw_docking_area_2 (Utilities|Casting|CastToW_DockingArea (UserInterface|GetWidget (Variables|Default|GetDockingAreaWidget))))
        (Default|ShowStopBox _asw_docking_area_2)))))

(fn ConstructionScript)

(fn UpdateHighlighterMaterial
  (params (New%20Colour :type Linear%20Color%20Structure))
  (bind _returnvalue (Rendering|Material|CreateDynamicMaterialInstance (Variables|Default|GetDockingAreaMesh) 0 "/Game/Gameplay/DockingArea/Materials/M_MasterHightlight_Instance.M_MasterHightlight_Instance" "None" :!class /Script/Engine.PrimitiveComponent))
  (Rendering|Material|SetVectorParameterValue _returnvalue "HighlighterColour" New%20Colour :!class /Script/Engine.MaterialInstanceDynamic))

(fn PowerboatIsStopped
  (return (Math|Float|NearlyEqual(Float) (Math|Vector|VectorLength (Transformation|GetVelocity (Variables|Default|GetPowerboat))) 0.0 0.1)))