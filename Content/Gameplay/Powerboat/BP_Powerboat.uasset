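; Player-controlled powerboat that adds boat and UI input mappings, handles the pause input, and drives movement, spray effects and engine audio.
; Each tick it passes forward and turn input to BoatControllerComp and mutes the engine below a speed threshold in MPH.
; Move input toggles the wake and side sprays, with side sprays only on positive input.
; A BoatSound timeline ramps engine pitch up, reversing on release.
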(event Input|EnhancedActionEvents|EnhancedInputActionIA_Boat_Move
  (params (ActionValue :type Float%20%28double-precision%29) (ElapsedSeconds :type Float%20%28double-precision%29) (TriggeredSeconds :type Float%20%28double-precision%29) (InputAction :type Input%20Action%20Object%20Reference :default "/Game/Input/IA_Boat_Move.IA_Boat_Move"))
  (:Triggered
    (CallFunction|CreateBoatSpray true ActionValue)
    (bind _boatpitchmultiplier (Timeline|BoatSound Play)
      (:Update
        (Audio|Components|Audio|SetPitchMultiplier (Variables|Default|GetSQ_BoatEngine) _boatpitchmultiplier))))
  (:Completed
    (CallFunction|CreateBoatSpray false ActionValue)
    (Timeline|BoatSound Reverse)))

(event Input|EnhancedActionEvents|EnhancedInputActionIA_Pause
  (params (ActionValue :type Boolean) (ElapsedSeconds :type Float%20%28double-precision%29) (TriggeredSeconds :type Float%20%28double-precision%29) (InputAction :type Input%20Action%20Object%20Reference :default "/Game/Input/IA_Pause.IA_Pause"))
  ;[0 0 0] Pausing Game
  (if (not (Game|IsGamePaused))
    (Default|CallPauseGame)))

(event EventBeginPlay
  ;[0 0 0] Setting up controls
  (Utilities|FlowControl|Delay 0.2)
  (Input|AddMappingContext (PlayerController|LocalPlayerSubsystems|GetEnhancedInputLocalPlayerSubsystem (Game|GetPlayerController 0)) "/Game/Input/IMC_BoatControls.IMC_BoatControls" 0 "(bIgnoreAllPressedKeysUntilRelease=True,bForceImmediately=False,bNotifyUserSettings=False)")
  (Input|AddMappingContext (PlayerController|LocalPlayerSubsystems|GetEnhancedInputLocalPlayerSubsystem (Game|GetPlayerController 0)) "/Game/Input/IMC_UI.IMC_UI" 0 "(bIgnoreAllPressedKeysUntilRelease=True,bForceImmediately=False,bNotifyUserSettings=False)")
  (CallFunction|CreateBoatSpray false 0.0)
  (Audio|Components|Audio|SetPitchMultiplier (Variables|Default|GetSQ_BoatEngine) 0.0))

(event Collision|EventActorBeginOverlap
  (params (OtherActor :type Actor%20Object%20Reference)))

(event EventTick
  (params (DeltaSeconds :type Float%20%28single-precision%29))
  (bind _sq_boatengine (Variables|Default|GetSQ_BoatEngine))
  ;[0 0 0] Updatating Boat Component Forward and Turn Input
  (Class|BoatControllerComponent|SetInputs (Variables|Default|GetboatControllerComp) (Input|EnhancedActionValues|GetIA_Boat_Move) (Input|EnhancedActionValues|GetIA_Boat_Turn))
  (bind _current_speed (CallFunction|GetSpeed))
  (if (< _current_speed 2.0)
    (Audio|Components|Audio|SetVolumeMultiplier _sq_boatengine 0.0 :!class /Script/Engine.AudioComponent)
    (else
      (Audio|Components|Audio|SetVolumeMultiplier _sq_boatengine 1e+01 :!class /Script/Engine.AudioComponent))))

(fn ConstructionScript)

(fn CreateBoatSpray
  (params (Play :type Boolean) (ForwardDirection :type Float%20%28double-precision%29))
  (bind _boatwake (Variables|Default|GetBoatWake))
  (bind _boatsprayleft (Variables|Default|GetBoatSprayLeft))
  (bind _boatsprayright (Variables|Default|GetBoatSprayRight))
  (if Play
    (Components|Activation|Activate _boatsprayleft false)
    (Components|Activation|Activate _boatsprayright false)
    (Components|Activation|Activate _boatwake false)
    (Development|PrintString (Utilities|String|ToString(Float) ForwardDirection))
    (if (not (> ForwardDirection 0.0))
      (Components|Activation|Deactivate (Variables|Default|GetBoatSprayLeft))
      (Components|Activation|Deactivate (Variables|Default|GetBoatSprayRight)))
    (else
      (Components|Activation|Deactivate _boatsprayleft)
      (Components|Activation|Deactivate _boatsprayright)
      (Components|Activation|Deactivate _boatwake))))

(fn GetSpeed
  ;[0 0 0] Returning Speed (MPH)
  (return (* (Math|Vector|VectorLength (Transformation|GetVelocity)) 0.0224)))

(fn IsMoving
  (bind _current_speed (CallFunction|GetSpeed))
  (return (not (Math|Float|NearlyEqual(Float) _current_speed 0.0 0.1))))