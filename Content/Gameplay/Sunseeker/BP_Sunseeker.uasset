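; Sunseeker actor that flies along a chained cubic Bezier path defined by its Points array.
; BeginPlay converts the points to world space, then a timeline drives location and tangent-facing rotation through each segment, stepping three points at a time.
; Bezier positions come from nested lerps, and rotation from sampling a nearby point on the curve.
; Debug helpers draw the path, including from the construction script when ShowDebug is set.
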(event EventBeginPlay
  (bind _points (Variables|Default|GetPoints))
  (Utilities|FlowControl|Sequence
    (:then_0
      (Utilities|Array|Insert :TargetArray _points)
      (for (_array_element _array_index) _points
        (Utilities|Array|SetArrayElem _points _array_index (Math|Transform|TransformLocation (Transformation|GetActorTransform) _array_element))))
    (:then_1
      (if (CallFunction|IsNextTravelIndexValid (Variables|Default|GetPoints) (Variables|Default|GetStartTravelIndex))
        (Utilities|FlowControl|Delay 0.2)
        (Components|Timeline|PlayfromStart (Variables|Default|GetTimeline_Lerp))))))

(fn ConstructionScript
  (if (Variables|Default|GetShowDebug)
    (CallFunction|DrawCurveforSeconds 0.02)))

(fn GetLocationBezier
  (params (StartPoint :type Vector) (AnchorStart :type Vector) (AnchorEnd :type Vector) (EndPoint :type Vector) (Time :type Float%20%28double-precision%29))
  (Utilities|FlowControl|Sequence
    (:then_0
      (LocalVariables|SetTemp_A (Math|Vector|Lerp(Vector) StartPoint AnchorStart Time))
      (LocalVariables|SetTemp_B (Math|Vector|Lerp(Vector) AnchorStart AnchorEnd Time))
      (LocalVariables|SetTemp_C (Math|Vector|Lerp(Vector) AnchorEnd EndPoint Time)))
    (:then_1
      (LocalVariables|SetTemp%20D (Math|Vector|Lerp(Vector) (LocalVariables|GetTemp_A) (LocalVariables|GetTemp_B) Time))
      (LocalVariables|SetTemp%20E (Math|Vector|Lerp(Vector) (LocalVariables|GetTemp_B) (LocalVariables|GetTemp_C) Time)))
    (:then_2
      (return (Math|Vector|Lerp(Vector) (LocalVariables|GetTemp%20D) (LocalVariables|GetTemp%20E) Time)))))

(fn GetRotatorBezier
  (params (StartPoint :type Vector) (Anchor%20Start :type Vector) (Anchor%20End :type Vector) (EndPoint :type Vector) (Time :type Float%20%28double-precision%29))
  (bind _returnvalue (+ Time -0.001))
  (LocalVariables|SetTempCurrent (CallFunction|GetLocationBezier StartPoint Anchor%20Start Anchor%20End EndPoint Time))
  (if (Math|Float|InRange(Float) _returnvalue 0.0 1.0)
    (return (Math|Conversions|RotationFromXVector (Math|Vector|Normalize (- (LocalVariables|GetTempCurrent) (CallFunction|GetLocationBezier StartPoint Anchor%20Start Anchor%20End EndPoint _returnvalue)))))
    (else
      (return (Math|Conversions|RotationFromXVector (Math|Vector|Normalize (- (CallFunction|GetLocationBezier StartPoint Anchor%20Start Anchor%20End EndPoint (+ Time 0.001)) (LocalVariables|GetTempCurrent))))))))

(fn UpdatetoWorldVector
  (params (InVector :type Vector%20%28by%20ref%29))
  (|SetBy-RefVar InVector (Math|Transform|TransformLocation (Transformation|GetActorTransform) InVector)))

(fn IsNextTravelIndexValid
  (params (In%20Points :type Array%20of%20Vectors) (In%20Start%20Index :type Integer))
  (for _index (range 1 3)
    (if (not (Utilities|Array|IsValidIndex (Variables|Default|GetPoints) (+ In%20Start%20Index _index)))
      (return false)))
  (return true))

(fn DrawCurveforSeconds
  (params (InDuration :type Float%20%28double-precision%29))
  (Utilities|FlowControl|Sequence
    (:then_0
      ;[1 1 1] Collect simulated points
      (Utilities|IsValid (Game|GetGameInstance)
        (:Is%20Valid
          (for _array_element (Variables|Default|GetPoints)
            (Utilities|Array|Add (LocalVariables|GetTemp%20Sim%20Points) _array_element)))
        (:Is%20Not%20Valid
          (Utilities|Array|Add (LocalVariables|GetTemp%20Sim%20Points) (Transformation|GetActorLocation))
          (for _array_element_2 (Variables|Default|GetPoints)
            (Utilities|Array|Add (LocalVariables|GetTemp%20Sim%20Points) (Math|Transform|TransformLocation (Transformation|GetActorTransform) _array_element_2))))))
    (:then_1
      (LocalVariables|SetTemp%20Debug%20Start (Utilities|Array|Get(acopy) (LocalVariables|GetTemp%20Sim%20Points)))
      (while (CallFunction|IsNextTravelIndexValid (LocalVariables|GetTemp%20Sim%20Points) (LocalVariables|GetTemp%20Start%20Index))
        (Utilities|FlowControl|Sequence
          (:then_0
            (while (Math|Float|InRange(Float) (LocalVariables|GetTemp%20Time) 0.0 1.0)
              (Utilities|FlowControl|Sequence
                (:then_0
                  (bind _output_get (LocalVariables|SetTemp%20Debug%20End (CallFunction|GetLocationBezier (.Start (Utilities|GetBezierPoints (LocalVariables|GetTemp%20Sim%20Points) (LocalVariables|GetTemp%20Start%20Index))) (.AnchorStart (Utilities|GetBezierPoints (LocalVariables|GetTemp%20Sim%20Points) (LocalVariables|GetTemp%20Start%20Index))) (.AnchorEnd (Utilities|GetBezierPoints (LocalVariables|GetTemp%20Sim%20Points) (LocalVariables|GetTemp%20Start%20Index))) (.End (Utilities|GetBezierPoints (LocalVariables|GetTemp%20Sim%20Points) (LocalVariables|GetTemp%20Start%20Index))) (LocalVariables|GetTemp%20Time))))
                  (Rendering|Debug|DrawDebugLine (LocalVariables|GetTemp%20Debug%20Start) _output_get "(R=1.000000,G=0.000000,B=0.024231,A=1.000000)" InDuration 2e+01)
                  (LocalVariables|SetTemp%20Debug%20Start (LocalVariables|GetTemp%20Debug%20End)))
                (:then_1
                  (LocalVariables|SetTemp%20Time (+ (LocalVariables|GetTemp%20Time) 0.01))))))
          (:then_1
            (LocalVariables|SetTemp%20Start%20Index (+ (LocalVariables|GetTemp%20Start%20Index) 3))
            (LocalVariables|SetTemp%20Time 0.0)))))))

(fn DrawCurve
  (CallFunction|DrawCurveforSeconds 2.0))