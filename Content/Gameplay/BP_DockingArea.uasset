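; Docking zone that detects a BP_Powerboat and tracks a countdown while the boat is stationary.
; Mesh overlap stores the boat, toggles the docking widget and recolours the highlighter green inside or red on exit through a new dynamic material instance.
; Tick steps and prints the countdown when the stored boat's speed is near zero.
; Exit keeps the boat reference, so the countdown can also run outside the zone.
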(event OnComponentBeginOverlap(DockingAreaMesh)
  (params (OverlappedComponent :type Primitive%20Component%20Object%20Reference) (OtherActor :type Actor%20Object%20Reference) (OtherComp :type Primitive%20Component%20Object%20Reference) (OtherBodyIndex :type Integer) (bFromSweep :type Boolean) (SweepResult :type Hit%20Result%20Structure%20%28by%20ref%29))
  (bind _asbp_powerboat (Utilities|Casting|CastToBP_Powerboat OtherActor))
  (Variables|Default|SetPowerboat _asbp_powerboat)
  (CallFunction|UpdateHighlighterMaterial "(R=0.045569,G=1.000000,B=0.000000,A=1.000000)")
  (Development|SetHiddeninGame (Variables|Default|GetDockingAreaWidget) false false))

(event OnComponentEndOverlap(DockingAreaMesh)
  (params (OverlappedComponent :type Primitive%20Component%20Object%20Reference) (OtherActor :type Actor%20Object%20Reference) (OtherComp :type Primitive%20Component%20Object%20Reference) (OtherBodyIndex :type Integer))
  (bind _asbp_powerboat (Utilities|Casting|CastToBP_Powerboat OtherActor))
  (Variables|Default|SetPowerboat _asbp_powerboat)
  (CallFunction|UpdateHighlighterMaterial "(R=1.000000,G=0.007519,B=0.000000,A=1.000000)")
  (Development|SetHiddeninGame (Variables|Default|GetDockingAreaWidget) true false))

(event EventBeginPlay
  (Development|SetHiddeninGame (Variables|Default|GetDockingAreaWidget) true false))

(event Collision|EventActorBeginOverlap
  (params (OtherActor :type Actor%20Object%20Reference)))

(event EventTick
  (params (DeltaSeconds :type Float%20%28single-precision%29))
  (Utilities|IsValid (Variables|Default|GetPowerboat)
    (:Is%20Valid
      (if (CallFunction|PowerboatIsStopped)
        (bind _output_get (Variables|Default|SetCountdownTimer (Math|Interpolation|FInterptoConstant (Variables|Default|GetCountdownTimer) 0.0 DeltaSeconds 2.0)))
        (Development|PrintString (Utilities|String|Append "Coutndown" (Utilities|String|ToString(Float) _output_get)))))))

(fn ConstructionScript)

(fn UpdateHighlighterMaterial
  (params (New%20Colour :type Linear%20Color%20Structure))
  (bind _returnvalue (Rendering|Material|CreateDynamicMaterialInstance (Variables|Default|GetDockingAreaMesh) 0 "/Game/MasterMaterials/M_MasterHightlight_Instance.M_MasterHightlight_Instance" "None" :!class /Script/Engine.PrimitiveComponent))
  (Rendering|Material|SetVectorParameterValue _returnvalue "HighlighterColour" New%20Colour :!class /Script/Engine.MaterialInstanceDynamic))

(fn PowerboatIsStopped
  (return (Math|Float|NearlyEqual(Float) (Math|Vector|VectorLength (Transformation|GetVelocity (Variables|Default|GetPowerboat))) 0.0 0.1)))